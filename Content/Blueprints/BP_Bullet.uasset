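; BP_Bullet is a projectile that kills the player or armed enemies on impact.
; Its first mesh hit swaps the victim's skeletal mesh to a full-ragdoll physics asset and calls Death on BP_IKPlayer or BP_EnemyWithWeapon.
; It then applies an impulse at the impact point to any simulating body, pushing the hit bone away from the bullet.
; Finally it ignores the Pawn channel and destroys itself after a short delay.
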(event `self.BulletMesh.OnComponentHit`
  (params (HitComponent :type "PrimitiveComponent Object Reference") (OtherActor :type "Actor Object Reference") (OtherComp :type "PrimitiveComponent Object Reference") (NormalImpulse :type "Vector Structure") (Hit :type "HitResult Structure (by ref)"))
  (bind (_bblockinghit _binitialoverlap _time _distance _location _impactpoint _normal _impactnormal _physmat _hitactor _hitcomponent _hitbonename) (`GameplayStatics.BreakHitResult` Hit))
  (bind _returnvalue (`self.GetComponentByClass` OtherActor "/Script/Engine.SkeletalMeshComponent"))
  (`/Engine/EditorBlueprintResources/StandardMacros.DoOnce` false
    (:`Completed`
      (`|ExecutionSequence`
        (:`then_0`
          (`/Engine/EditorBlueprintResources/StandardMacros.IsValid` _returnvalue
            (:`Is Valid`
              (`SkinnedMeshComponent.SetPhysicsAsset` _returnvalue "/Game/Meshes/FlatFeldHuman_PhysicsAsset_FullRagdoll.FlatFeldHuman_PhysicsAsset_FullRagdoll" false)
              (bind _asbp_ikplayer (cast `/Game/Blueprints/BP_IKPlayer` OtherActor)
                (:`then`
                  (`/Game/Blueprints/BP_IKPlayer.Death` _asbp_ikplayer))
                (:`CastFailed`
                  (bind _asbp_enemy_with_weapon (cast `/Game/Blueprints/BP_EnemyWithWeapon` OtherActor))
                  (`/Game/Blueprints/BP_EnemyWithWeapon.Death` _asbp_enemy_with_weapon))))))
        (:`then_1`
          (if (`SceneComponent.IsSimulatingPhysics` OtherComp _hitbonename)
            (`PrimitiveComponent.AddImpulseAtLocation` OtherComp (* (`KismetMathLibrary.Normal` (- (`SceneComponent.GetSocketLocation` OtherComp _hitbonename) (`self.K2_GetActorLocation`))) 10000.0) _impactpoint _hitbonename)))
        (:`then_2`
          (`PrimitiveComponent.SetCollisionResponseToChannel` (`self.BulletMesh`) "ECC_Pawn" "ECR_Ignore")
          (`KismetSystemLibrary.Delay` 2.0)
          (`self.K2_DestroyActor`))))))

(fn `UserConstructionScript`)