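; Gun actor whose Shoot event plays an attenuated pistol sound and fires a physics-driven BP_Bullet from the ShootFrom component.
; The spawned bullet mesh is rotated, launched by a forward impulse, then scaled down.
; The Player flag picks which collision channel the bullet ignores: Pawn for player shots, a custom game channel (GameTraceChannel1) otherwise.
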(event `Shoot`
  (params (Player :type Boolean))
  (bind _shootfrom (`self.ShootFrom`))
  (`GameplayStatics.PlaySoundAtLocation` "/Game/Sound/Gun_Pistol_Shot06.Gun_Pistol_Shot06" (`self.K2_GetActorLocation`) (struct) 1.0 1.0 0.0 "/Game/Sound/gunattenuation.gunattenuation" null null null)
  (bind _returnvalue (`|SpawnActorFromClass` "/Game/Blueprints/BP_Bullet.BP_Bullet_C" (`SceneComponent.K2_GetComponentToWorld` _shootfrom) "Undefined" "OverrideRootScale" null null))
  (bind _bulletmesh (`/Game/Blueprints/BP_Bullet.BulletMesh` _returnvalue))
  (`SceneComponent.K2_AddWorldRotation` _bulletmesh (struct :`Pitch` 90.0) false false)
  (`PrimitiveComponent.AddImpulse` _bulletmesh (* (`SceneComponent.GetForwardVector` _shootfrom) 100000.0) "None" false)
  (`SceneComponent.SetWorldScale3D` _bulletmesh (0.1 0.1 0.1))
  (if Player
    (`PrimitiveComponent.SetCollisionResponseToChannel` _bulletmesh "ECC_Pawn" "ECR_Ignore")
    (else
      (`PrimitiveComponent.SetCollisionResponseToChannel` _bulletmesh "ECC_GameTraceChannel1" "ECR_Ignore"))))

(fn `UserConstructionScript`)