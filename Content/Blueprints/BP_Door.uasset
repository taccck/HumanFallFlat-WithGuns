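; BP_Door is a two-panel door that opens and closes according to a button state.
; The Buttonactive event snaps RightDoor and LeftDoor to their Destination components when active, or to their Arrow components when inactive.
; Movement is instant and unswept, with no interpolation.
; BeginPlay enables player 0 input, though the graph handles no input events.
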(event `self.ReceiveBeginPlay`
  (`self.EnableInput` (`GameplayStatics.GetPlayerController` 0)))

(event `/Game/Interfaces/Buttoninterface.buttonactive`
  (params (isactive :type Boolean))
  (if isactive
    (`|ExecutionSequence`
      (:`then_0`
        ;[1 1 1] open door
        (`SceneComponent.K2_SetWorldLocation` (`self.right door`) (`SceneComponent.K2_GetComponentLocation` (`self.destination right`)) false false))
      (:`then_1`
        (`SceneComponent.K2_SetWorldLocation` (`self.left door`) (`SceneComponent.K2_GetComponentLocation` (`self.destination left`)) false false)))
    (else
      (`|ExecutionSequence`
        (:`then_0`
          ;[1 1 1] open door
          (`SceneComponent.K2_SetWorldLocation` (`self.right door`) (`SceneComponent.K2_GetComponentLocation` (`self.Arrow right`)) false false))
        (:`then_1`
          (`SceneComponent.K2_SetWorldLocation` (`self.left door`) (`SceneComponent.K2_GetComponentLocation` (`self.Arrow left`)) false false))))))

(fn `UserConstructionScript`)